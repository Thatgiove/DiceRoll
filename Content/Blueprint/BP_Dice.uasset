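; BP_Dice is a die actor that reports which face value it shows and how fast it is moving.
; GetDiceFace loops through six face components and returns the first component tag, as an integer, of the first face aligned with the Normal component.
; Alignment is a dot product of normalized forward vectors against a fixed threshold, so it tolerates tilt.
; GetDiceVelocity returns the speed of DiceMesh.
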(fn ConstructionScript)

(fn CalculateifVectorsAreParallel
  (params (DiceFace :type Scene%20Component%20Object%20Reference))
  (if (>= (Math|Vector|DotProduct (Math|Vector|Normalize (Math|Vector|GetForwardVector DiceFace)) (Math|Vector|Normalize (Math|Vector|GetForwardVector (Variables|Default|GetNormal)))) 0.7)
    (return true)
    (else
      (return false))))

(fn GetDiceFace
  (bind _array_element (Utilities|Array|ForEachLoopwithBreak (Utilities|Array|MakeArray (Variables|Default|GetFace_1) (Variables|Default|GetFace_2) (Variables|Default|GetFace_3) (Variables|Default|GetFace_4) (Variables|Default|GetFace_5) (Variables|Default|GetFace_6)))
    (:LoopBody
      (bind _areparallel (CallFunction|CalculateifVectorsAreParallel _array_element))
      (if _areparallel
        (return (Math|Conversions|ToInteger(Byte) (Utilities|String|ToString(Name) (Utilities|Array|Get(acopy) (Variables|/Script/Engine.ActorComponent|GetComponentTags _array_element)))))))))

(fn GetDiceVelocity
  (return (Math|Vector|VectorLength (Transformation|GetComponentVelocity (Variables|Default|GetDiceMesh)))))