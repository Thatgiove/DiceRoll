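; BP_DiceRollGameModeBase is a dice game mode Blueprint that records roll totals and reports them to the HUD.
; AddSumToScoreArray appends each total to PreviousRoll until it holds six entries, ignoring later totals, and runs an empty loop over the array.
; After each append it finds the top-level DiceGameHUD through GetAllWidgetsOfClass and passes the newest entry to UpdateScore, without checking that a widget exists.
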(fn ConstructionScript)

(fn AddSumtoScoreArray
  (params (Total :type Integer))
  (bind _previousroll (Variables|Default|GetPreviousRoll))
  (if (< (Utilities|Array|Length _previousroll) 6)
    (Utilities|Array|Add _previousroll Total)
    (for _array_element _previousroll
      _)
    ;[1 1 1] Update HUD score con l'ultimo elemento
    (bind _foundwidgets (Widget|GetAllWidgetsOfClass "/Game/UI/DiceGameHUD.DiceGameHUD_C" true))
    (Default|UpdateScore (Utilities|Array|Get(acopy) _foundwidgets) (Utilities|Array|Get(acopy) _previousroll (Utilities|Array|LastIndex _previousroll)))))