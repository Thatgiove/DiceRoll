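; Deprecated interactable object that shows character proximity and gates play in the dice roll game.
; Two sphere colliders swap the mesh material between default, external and internal states as a character enters or leaves each range.
; Entering the inner sphere sets CanPlay on BP_DiceRollGameModeBase and briefly shows a text render; leaving it clears the flag.
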(event OnComponentBeginOverlap(InternalSphereCollider)
  (params (OverlappedComponent :type Primitive%20Component%20Object%20Reference) (OtherActor :type Actor%20Object%20Reference) (OtherComp :type Primitive%20Component%20Object%20Reference) (OtherBodyIndex :type Integer) (bFromSweep :type Boolean) (SweepResult :type Hit%20Result%20Structure%20%28by%20ref%29))
  (bind _textrender (Variables|Default|GetTextRender))
  ;[1 1 1] Overlapping Event
  (Utilities|Casting|CastToCharacter OtherActor)
  (Rendering|Material|SetMaterial (Variables|Default|GetStaticMesh) 0 (Variables|Default|GetInternalMaterial))
  (bind _asbp_dice_roll_game_mode_base (Utilities|Casting|CastToBP_DiceRollGameModeBase (Game|GetGameMode)))
  (Variables|/Game/Blueprint/GameMode/BP_DiceRollGameModeBase.BP_DiceRollGameModeBase_C|SetbCanPlay _asbp_dice_roll_game_mode_base true)
  (Rendering|SetVisibility _textrender true false)
  (Utilities|FlowControl|Delay 2.0)
  (Rendering|SetVisibility _textrender false false))

(event OnComponentBeginOverlap(ExternalSphereCollider)
  (params (OverlappedComponent :type Primitive%20Component%20Object%20Reference) (OtherActor :type Actor%20Object%20Reference) (OtherComp :type Primitive%20Component%20Object%20Reference) (OtherBodyIndex :type Integer) (bFromSweep :type Boolean) (SweepResult :type Hit%20Result%20Structure%20%28by%20ref%29))
  ;[1 1 1] Overlapping Event
  (Utilities|Casting|CastToCharacter OtherActor)
  (Rendering|Material|SetMaterial (Variables|Default|GetStaticMesh) 0 (Variables|Default|GetExternalMaterial)))

(event OnComponentEndOverlap(ExternalSphereCollider)
  (params (OverlappedComponent :type Primitive%20Component%20Object%20Reference) (OtherActor :type Actor%20Object%20Reference) (OtherComp :type Primitive%20Component%20Object%20Reference) (OtherBodyIndex :type Integer))
  ;[1 1 1] Overlapping Event
  (Utilities|Casting|CastToCharacter OtherActor)
  (Rendering|Material|SetMaterial (Variables|Default|GetStaticMesh) 0 (Variables|Default|GetDefaultMaterial)))

(event OnComponentEndOverlap(InternalSphereCollider)
  (params (OverlappedComponent :type Primitive%20Component%20Object%20Reference) (OtherActor :type Actor%20Object%20Reference) (OtherComp :type Primitive%20Component%20Object%20Reference) (OtherBodyIndex :type Integer))
  ;[1 1 1] Overlapping Event
  (Utilities|Casting|CastToCharacter OtherActor)
  (Rendering|Material|SetMaterial (Variables|Default|GetStaticMesh) 0 (Variables|Default|GetExternalMaterial))
  (bind _asbp_dice_roll_game_mode_base (Utilities|Casting|CastToBP_DiceRollGameModeBase (Game|GetGameMode)))
  (Variables|/Game/Blueprint/GameMode/BP_DiceRollGameModeBase.BP_DiceRollGameModeBase_C|SetbCanPlay _asbp_dice_roll_game_mode_base false))

(fn ConstructionScript)